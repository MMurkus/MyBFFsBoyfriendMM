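; BP_Door is an interactable hinged door that the player swings open with IA_Interact and that closes itself again.
; A Box overlap enables input and shows a Widget only while the player character is inside.
; A Timeline lerps the Hinge toward DoorEndRotation, disabling Door collision during motion and restoring it on finish.
; The Timeline reverses after a delay, triggered on finishing or when the player leaves the Box.
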(event OnComponentBeginOverlap(Box)
  (params (OverlappedComponent :type Primitive%20Component%20Object%20Reference) (OtherActor :type Actor%20Object%20Reference) (OtherComp :type Primitive%20Component%20Object%20Reference) (OtherBodyIndex :type Integer) (bFromSweep :type Boolean) (SweepResult :type Hit%20Result%20Structure%20%28by%20ref%29))
  (if (== OtherActor (Game|GetPlayerCharacter 0))
    (Input|EnableInput (Game|GetPlayerController 0))
    (Rendering|SetVisibility (Variables|Default|GetWidget) true false)))

(event OnComponentEndOverlap(Box)
  (params (OverlappedComponent :type Primitive%20Component%20Object%20Reference) (OtherActor :type Actor%20Object%20Reference) (OtherComp :type Primitive%20Component%20Object%20Reference) (OtherBodyIndex :type Integer))
  (if (== OtherActor (Game|GetPlayerCharacter 0))
    (Input|DisableInput (Game|GetPlayerController 0))
    (Rendering|SetVisibility (Variables|Default|GetWidget) false false)
    (Utilities|FlowControl|Delay 2.0)
    (bind _doorrotate (Timeline|Timeline Reverse)
      (:Update
        (Collision|SetCollisionEnabled (Variables|Default|GetDoor) "NoCollision")
        (Transformation|SetRelativeRotation (Variables|Default|GetHinge) (Math|Rotator|Lerp(Rotator) "0, 0, 0" (Variables|Default|GetDoorEndRotation) _doorrotate) false false)
        (Utilities|FlowControl|Delay 2.0))
      (:Finished
        (Collision|SetCollisionEnabled (Variables|Default|GetDoor) "QueryAndPhysics")
        (Utilities|FlowControl|Delay 2.0)
        (Timeline|Timeline Reverse)))))

(event Input|EnhancedActionEvents|EnhancedInputActionIA_Interact
  (params (ActionValue :type Boolean) (ElapsedSeconds :type Float%20%28double-precision%29) (TriggeredSeconds :type Float%20%28double-precision%29) (InputAction :type Input%20Action%20Object%20Reference :default "/Game/FirstPerson/Input/Actions/IA_Interact.IA_Interact"))
  (bind _doorrotate (Timeline|Timeline Play)
    (:Update
      (Collision|SetCollisionEnabled (Variables|Default|GetDoor) "NoCollision")
      (Transformation|SetRelativeRotation (Variables|Default|GetHinge) (Math|Rotator|Lerp(Rotator) "0, 0, 0" (Variables|Default|GetDoorEndRotation) _doorrotate) false false)
      (Utilities|FlowControl|Delay 2.0))
    (:Finished
      (Collision|SetCollisionEnabled (Variables|Default|GetDoor) "QueryAndPhysics")
      (Utilities|FlowControl|Delay 2.0)
      (Timeline|Timeline Reverse))))

(event EventBeginPlay)

(event Collision|EventActorBeginOverlap
  (params (OtherActor :type Actor%20Object%20Reference)))

(event EventTick
  (params (DeltaSeconds :type Float%20%28single-precision%29)))

(fn ConstructionScript)
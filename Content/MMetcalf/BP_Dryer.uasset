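; Interactable dryer actor that shows a prompt widget and enables input while the player is inside its box, unless it is running.
; Interact sets IsRunning, then joins the BeginPlay chain, which hides the widget and counts TotalInteractions, printing a completion message at two.
; BeginPlay consumes the DoOnce before the delayed IsRunning reset, so presses never restart that timer.
; NewFunction also clears IsRunning.
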(event OnComponentBeginOverlap(Box)
  (params (OverlappedComponent :type Primitive%20Component%20Object%20Reference) (OtherActor :type Actor%20Object%20Reference) (OtherComp :type Primitive%20Component%20Object%20Reference) (OtherBodyIndex :type Integer) (bFromSweep :type Boolean) (SweepResult :type Hit%20Result%20Structure%20%28by%20ref%29))
  (if (== OtherActor (Game|GetPlayerCharacter 0))
    (if (not (Variables|Default|GetisRunning?))
      (Input|EnableInput (Game|GetPlayerController 0))
      (Rendering|SetVisibility (Variables|Default|GetWidget) true false))))

(event OnComponentEndOverlap(Box)
  (params (OverlappedComponent :type Primitive%20Component%20Object%20Reference) (OtherActor :type Actor%20Object%20Reference) (OtherComp :type Primitive%20Component%20Object%20Reference) (OtherBodyIndex :type Integer))
  (if (== OtherActor (Game|GetPlayerCharacter 0))
    (Input|DisableInput (Game|GetPlayerController 0))
    (Rendering|SetVisibility (Variables|Default|GetWidget) false false)))

(event EventBeginPlay
  (Rendering|SetVisibility (Variables|Default|GetWidget) false false)
  (Math|Float|IncrementFloat (Variables|Default|GettotalInteractions)
    (:%20%20
      (Utilities|FlowControl|Sequence
        (:then_0
          (Utilities|FlowControl|DoOnce false
            (:Completed
              (Utilities|FlowControl|Delay 1e+01)
              (Variables|Default|SetisRunning? false))))
        (:then_1
          (if (== (Variables|Default|GettotalInteractions) 2.0)
            (Development|PrintString "Completed condition")))))))

(event Collision|EventActorBeginOverlap
  (params (OtherActor :type Actor%20Object%20Reference)))

(event EventTick
  (params (DeltaSeconds :type Float%20%28single-precision%29)))

(event EventNewFunction
  (Variables|Default|SetisRunning? false))

(event Input|ActionEvents|InputActionIA_Interact
  (params (Key :type Key%20Structure :default "None"))
  (:Pressed
    (Variables|Default|SetisRunning? true)
    (Rendering|SetVisibility (Variables|Default|GetWidget) false false)
    (Math|Float|IncrementFloat (Variables|Default|GettotalInteractions)
      (:%20%20
        (Utilities|FlowControl|Sequence
          (:then_0
            (Utilities|FlowControl|DoOnce false
              (:Completed
                (Utilities|FlowControl|Delay 1e+01)
                (Variables|Default|SetisRunning? false))))
          (:then_1
            (if (== (Variables|Default|GettotalInteractions) 2.0)
              (Development|PrintString "Completed condition"))))))))

(fn ConstructionScript)
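; BP_Disposal is a disposal point that destroys non-player actors entering its Box and counts them as body parts.
; At six it sets IsFull, stops accepting actors and prints a debug message.
; Tick separately checks whether the last overlapping actor is the player, then once pauses the game, shows the Wid_Really widget and enables the mouse cursor, regardless of IsFull.
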(event OnComponentBeginOverlap(Box)
  (params (OverlappedComponent :type Primitive%20Component%20Object%20Reference) (OtherActor :type Actor%20Object%20Reference) (OtherComp :type Primitive%20Component%20Object%20Reference) (OtherBodyIndex :type Integer) (bFromSweep :type Boolean) (SweepResult :type Hit%20Result%20Structure%20%28by%20ref%29))
  (if (not (Variables|Default|GetisFull?))
    (if (not (== OtherActor (Game|GetPlayerCharacter 0)))
      (Actor|DestroyActor OtherActor)
      (bind _result (Math|Float|IncrementFloat (Variables|Default|GetbodyParts))
        (:%20%20
          (Variables|Default|SetbodyParts _result)
          (if (== (Variables|Default|GetbodyParts) 6.0)
            (Variables|Default|SetisFull? true)
            (Development|PrintString "Body gon")))))))

(event EventBeginPlay)

(event Collision|EventActorBeginOverlap
  (params (OtherActor :type Actor%20Object%20Reference)))

(event EventTick
  (params (DeltaSeconds :type Float%20%28single-precision%29))
  (if (== (stale OnComponentBeginOverlap(Box) OtherActor) (Game|GetPlayerCharacter 0))
    (Utilities|FlowControl|DoOnce false
      (:Completed
        (Game|SetGamePaused true)
        (bind _returnvalue (UserInterface|CreateWidget "/Game/MMetcalf/Wid_Really.Wid_Really_C"))
        (UserInterface|Viewport|AddtoViewport _returnvalue 0)
        (Variables|/Script/Engine.PlayerController|SetbShowMouseCursor (Game|GetPlayerController 0) true)))))

(fn ConstructionScript)